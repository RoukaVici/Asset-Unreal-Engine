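; Motor Blueprint that represents one finger's vibration motor as a sphere, turning vibration on and off through key input or mouse clicks.
; Key press and release raise and lower a vibration counter, while a click toggles it between zero and one.
; Each tick, Vibrate clamps the counter, swaps the sphere's material, and sends start or stop commands for the motor index only on state changes, using sent flags.
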(event `self.ReceiveBeginPlay`
  ;[1 1 1] At the start of the program, stores the material of the object to use it later
  (set `self.currentMaterial` (`PrimitiveComponent.GetMaterial` (`self.Shere Shape`) 0)))

(event `self.ReceiveTick`
  (params (DeltaSeconds :type "Float (single-precision)"))
  (`|ExecutionSequence`
    (:`then_0`
      ;[1 1 1] Activates vibration mode for the finger
      (if (`PlayerController.WasInputKeyJustPressed` (`GameplayStatics.GetPlayerController` 0) (`self.key`))
        (set `self.vibrationCount` (+ (`self.vibrationCount`) 1))))
    (:`then_1`
      ;[1 1 1] Stops vibration mode for the finger
      (if (`PlayerController.WasInputKeyJustReleased` (`GameplayStatics.GetPlayerController` 0) (`self.key`))
        (set `self.vibrationCount` (- (`self.vibrationCount`) 1))))
    (:`then_2`
      (`self.Vibrate`))))

(event `self.Shere Shape.OnClicked`
  (params (TouchedComponent :type "PrimitiveComponent Object Reference") (ButtonPressed :type "Key Structure"))
  ;[1 1 1] Handle the OnClicked event
  (if (== (`self.vibrationCount`) 0)
    (set `self.vibrationCount` 1)
    (else
      (set `self.vibrationCount` 0))))

(fn `UserConstructionScript`)

(fn `Vibrate`
  (if (< (`self.vibrationCount`) 0)
    (set `self.vibrationCount` 0)
    (elif (> (`self.vibrationCount`) 0)
      ;[1 1 1] The finger started vibrating
      (if (== (`self.startSent`) false)
        (`PrimitiveComponent.SetMaterial` (`self.Shere Shape`) 0 (`self.activatedMaterial`))
        (`self.sendVibrationCommand` (`KismetMathLibrary.Conv_ByteToInt` (`self.Motor`)))
        (set `self.startSent` true)
        (set `self.stopSent` false))
      (else
        ;[1 1 1] The finger stopped vibrating
        (if (== (`self.stopSent`) false)
          (`PrimitiveComponent.SetMaterial` (`self.Shere Shape`) 0 (`self.currentMaterial`))
          (`self.stopVibrationCommand` (`KismetMathLibrary.Conv_ByteToInt` (`self.Motor`)))
          (set `self.stopSent` true)
          (set `self.startSent` false))))))