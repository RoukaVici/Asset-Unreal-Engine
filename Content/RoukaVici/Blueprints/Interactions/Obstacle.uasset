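; Obstacle is a player-movable actor that makes fingers vibrate on contact.
; Beginning or ending overlap with a Motor actor increments or decrements its VibrationCount, so simultaneous contacts are counted.
; Each tick polls the four arrow keys and moves the actor along world X and Y from the Cube's transform, scaled by Speed and delta time, without sweep.
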(event `self.ReceiveActorBeginOverlap`
  (params (OtherActor :type "Actor Object Reference"))
  ;[1 1 1] The finger has to vibrate
  (bind _asmotor (cast `/Game/RoukaVici/Blueprints/Motor` OtherActor))
  (set `/Game/RoukaVici/Blueprints/Motor.vibrationCount` (+ (`/Game/RoukaVici/Blueprints/Motor.vibrationCount` _asmotor) 1) _asmotor))

(event `self.ReceiveActorEndOverlap`
  (params (OtherActor :type "Actor Object Reference"))
  ;[1 1 1] The finger has to stop vibrating
  (bind _asmotor (cast `/Game/RoukaVici/Blueprints/Motor` OtherActor))
  (set `/Game/RoukaVici/Blueprints/Motor.vibrationCount` (- (`/Game/RoukaVici/Blueprints/Motor.vibrationCount` _asmotor) 1) _asmotor))

(event `self.ReceiveTick`
  (params (DeltaSeconds :type "Float (single-precision)"))
  (bind _returnvalue (`GameplayStatics.GetPlayerController` 0))
  (`|ExecutionSequence`
    (:`then_0`
      ;[1 1 1] Listens for key inputs
      (if (`PlayerController.IsInputKeyDown` _returnvalue "Up")
        (set `self.up` 1)
        (else
          (set `self.up` 0))))
    (:`then_1`
      (if (`PlayerController.IsInputKeyDown` _returnvalue "Down")
        (set `self.down` 1)
        (else
          (set `self.down` 0))))
    (:`then_2`
      (if (`PlayerController.IsInputKeyDown` _returnvalue "Left")
        (set `self.left` 1)
        (else
          (set `self.left` 0))))
    (:`then_3`
      (if (`PlayerController.IsInputKeyDown` _returnvalue "Right")
        (set `self.right` 1)
        (else
          (set `self.right` 0))))
    (:`then_4`
      (`self.K2_SetActorTransform` (`KismetMathLibrary.MakeTransform` (+ (.location (`SceneComponent.K2_GetComponentToWorld` (`self.Cube`))) (* (`KismetMathLibrary.MakeVector` (`KismetMathLibrary.Conv_IntToDouble` (- (`self.down`) (`self.up`))) (`KismetMathLibrary.Conv_IntToDouble` (- (`self.left`) (`self.right`)))) (* (`GameplayStatics.GetWorldDeltaSeconds`) (`self.speed`)))) (.rotation (`SceneComponent.K2_GetComponentToWorld` (`self.Cube`))) (.scale (`SceneComponent.K2_GetComponentToWorld` (`self.Cube`))))) ; Moves the obstacle
    )))

(fn `UserConstructionScript`)