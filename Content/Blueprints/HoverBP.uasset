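; HoverBP is a component-style Blueprint that makes its owning actor bob vertically.
; On BeginPlay it caches the owner's starting location and first mesh component, though the mesh is not used afterwards.
; Each Tick advances a time counter by Speed and offsets the owner's Z from that start by a cosine scaled by Amplitude.
; The motion is frame-rate dependent because the step ignores delta time.
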(event `self.ReceiveBeginPlay`
  (bind _returnvalue (`self.GetOwner`))
  (set `self.ParentMesh` (`|GetArrayItem` (`Actor.K2_GetComponentsByClass` _returnvalue "/Script/Engine.MeshComponent")))
  (set `self.parentPos` (`Actor.K2_GetActorLocation` _returnvalue)))

(event `self.ReceiveTick`
  (params (DeltaSeconds :type "Float (single-precision)"))
  (set `self.time` (+ (`self.time`) (`self.speed`)))
  (`Actor.K2_SetActorLocation` (`self.GetOwner`) (+ (`self.parentPos`) (`KismetMathLibrary.MakeVector` 0.0 0.0 (* (`KismetMathLibrary.Cos` (`self.time`)) (`self.amplitude`)))) false false))