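; Hover component that makes its owning actor bob up and down and spin.
; It caches the owner on BeginPlay, then each Tick adds a cosine-of-time vertical offset scaled by Speed and Amplitude to the current location.
; It also combines a Yaw step with the current rotation each Tick.
; Both changes accumulate per frame without delta-time scaling, so the motion depends on frame rate.
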(event `self.ReceiveBeginPlay`
  (set `self.owner` (`self.GetOwner`)))

(event `self.ReceiveTick`
  (params (DeltaSeconds :type "Float (single-precision)"))
  (`Actor.K2_SetActorLocation` (`self.owner`) (+ (`Actor.K2_GetActorLocation` (`self.owner`)) (`KismetMathLibrary.MakeVector` 0.0 0.0 (* (`KismetMathLibrary.Cos` (* (`GameplayStatics.GetTimeSeconds`) (`self.Speed`))) (`self.amplitude`)))) false false)
  (`Actor.K2_SetActorRotation` (`self.owner`) (`KismetMathLibrary.ComposeRotators` (`Actor.K2_GetActorRotation` (`self.owner`)) (`KismetMathLibrary.MakeRotator` 0.0 0.0 (`self.yaw`))) false))